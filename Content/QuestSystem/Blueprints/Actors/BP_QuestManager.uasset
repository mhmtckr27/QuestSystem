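; Quest manager actor that registers quests, tracks the selected one and guides the player to its current goal on the minimap.
; AddNewQuest spawns one actor per unique quest class, adds it to the quest list widget and selects it if first or immediate.
; Switching goals replaces the spawned BP_Goal marker.
; Player movement updates flat distance and arrow yaw, with paired DoOnce gates toggling arrow visibility around a distance threshold.
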(event Custom|OnSwitchGoal
  (bind _currentquest (Variables|QuestSystem|GetCurrentQuest))
  (Utilities|IsValid (Variables|QuestSystem|GetCurrentGoalActor)
    (:Is%20Valid
      (Actor|DestroyActor (Variables|QuestSystem|GetCurrentGoalActor)))
    (:Is%20Not%20Valid
      _))
  (bind _output_get (Variables|QuestSystem|SetCurrentGoal (Utilities|Array|Get(acopy) (.Goals (Utilities|Struct|BreakS_QuestInfo (Variables|/Game/QuestSystem/Blueprints/Actors/QuestActors/BP_QuestMaster.BP_QuestMaster_C|GetQuestInfo _currentquest))) (Variables|/Game/QuestSystem/Blueprints/Actors/QuestActors/BP_QuestMaster.BP_QuestMaster_C|GetSelectedSubgoalIndex _currentquest))))
  (if (.HasLocation (Utilities|Struct|BreakS_GoalLocation (.GoalLocation (Utilities|Struct|BreakS_GoalInfo _output_get))))
    (bind _returnvalue (Game|SpawnActorfromClass "/Game/QuestSystem/Blueprints/Actors/BP_Goal.BP_Goal_C" (Math|Transform|MakeTransform (.Location (Utilities|Struct|BreakS_GoalLocation (.GoalLocation (Utilities|Struct|BreakS_GoalInfo _output_get)))) "0, 0, 0" "1,1,1") "AlwaysSpawn" 0 (.HasRadius (Utilities|Struct|BreakS_GoalInfo _output_get)) (.Radius (Utilities|Struct|BreakS_GoalInfo _output_get)) (.RadiusColor (Utilities|Struct|BreakS_GoalInfo _output_get)) 0))
    (Variables|QuestSystem|SetCurrentGoalActor _returnvalue)
    (Rendering|Components|TextRender|SetText (Variables|/Game/QuestSystem/Widgets/WBP_Minimap.WBP_Minimap_C|GetDistanceText (Variables|/Game/QuestSystem/Widgets/WBP_MainWidget.WBP_MainWidget_C|GetWBP_Minimap (Variables|UI|GetMainWidget))) (Utilities|Text|ToText(Integer) (CallFunction|GetDistancetoGoal) false false))
    (CallFunction|UpdateDirectionArrow)
    (Widget|SetVisibility (Variables|/Game/QuestSystem/Widgets/WBP_Minimap.WBP_Minimap_C|GetDistanceBorder (Variables|/Game/QuestSystem/Widgets/WBP_MainWidget.WBP_MainWidget_C|GetWBP_Minimap (Variables|UI|GetMainWidget))) "HitTestInvisible")
    (Widget|SetVisibility (Variables|/Game/QuestSystem/Widgets/WBP_Minimap.WBP_Minimap_C|GetDirectionArrow (Variables|/Game/QuestSystem/Widgets/WBP_MainWidget.WBP_MainWidget_C|GetWBP_Minimap (Variables|UI|GetMainWidget))) (select (> (CallFunction|GetDistancetoGoal) (Variables|Default|GetShowDirectionArrowDistance)) "HitTestInvisible" "Hidden"))
    (else
      (Widget|SetVisibility (Variables|/Game/QuestSystem/Widgets/WBP_Minimap.WBP_Minimap_C|GetDirectionArrow (Variables|/Game/QuestSystem/Widgets/WBP_MainWidget.WBP_MainWidget_C|GetWBP_Minimap (Variables|UI|GetMainWidget))) "Hidden"))))

(event Custom|OnPlayerMove
  (bind _distance (CallFunction|GetDistancetoGoal))
  (bind _mainwidget (Variables|UI|GetMainWidget))
  (bind _wbp_minimap (Variables|/Game/QuestSystem/Widgets/WBP_MainWidget.WBP_MainWidget_C|GetWBP_Minimap _mainwidget))
  (bind _directionarrow (Variables|/Game/QuestSystem/Widgets/WBP_Minimap.WBP_Minimap_C|GetDirectionArrow _wbp_minimap))
  (Utilities|IsValid (Variables|QuestSystem|GetCurrentGoalActor)
    (:Is%20Valid
      (Rendering|Components|TextRender|SetText (Variables|/Game/QuestSystem/Widgets/WBP_Minimap.WBP_Minimap_C|GetDistanceText (Variables|/Game/QuestSystem/Widgets/WBP_MainWidget.WBP_MainWidget_C|GetWBP_Minimap (Variables|UI|GetMainWidget))) (Utilities|Text|ToText(Integer) _distance false false))
      (Math|Integer|CompareInt _distance (Variables|Default|GetShowDirectionArrowDistance)
        (:>
          _)
        (:==
          _)
        (:<
          (Utilities|FlowControl|DoOnce false :!label _label
            (:Completed
              (Widget|SetVisibility _directionarrow "Hidden")
              (goto _label_2 Reset)))))
      (CallFunction|UpdateDirectionArrow)
      (Utilities|FlowControl|DoOnce false :!label _label_2
        (:Completed
          (Widget|SetVisibility _directionarrow "HitTestInvisible")
          (goto _label Reset))))))

(event EventBeginPlay)

(fn ConstructionScript)

(fn SelectNewQuest
  (params (Quest :type BP%20Quest%20Master%20Object%20Reference) (Goal :type WBP%20Goal%20Object%20Reference))
  (Utilities|IsValid (Variables|QuestSystem|GetCurrentQuest)
    (:Is%20Valid
      (Widget|SetIsEnabled (Variables|/Game/QuestSystem/Widgets/WBP_Quest.WBP_Quest_C|GetQuestName (Variables|/Game/QuestSystem/Blueprints/Actors/QuestActors/BP_QuestMaster.BP_QuestMaster_C|GetQuestWidget (Variables|QuestSystem|GetCurrentQuest))) false)
      (Default|SelectGoal (Variables|/Game/QuestSystem/Blueprints/Actors/QuestActors/BP_QuestMaster.BP_QuestMaster_C|GetQuestWidget (Variables|QuestSystem|GetCurrentQuest))))
    (:Is%20Not%20Valid
      _))
  (bind _output_get (Variables|QuestSystem|SetCurrentQuest Quest))
  (Default|OnQuestSelected (Variables|/Game/QuestSystem/Blueprints/Actors/QuestActors/BP_QuestMaster.BP_QuestMaster_C|GetQuestWidget _output_get) Goal)
  (return))

(fn AddNewQuest
  (params (QuestClass :type BP%20Quest%20Master%20Class%20Reference) (ShouldStartImmediately :type Boolean))
  (bind _mainwidget (Variables|UI|GetMainWidget))
  (bind _wbp_questlist (Variables|/Game/QuestSystem/Widgets/WBP_MainWidget.WBP_MainWidget_C|GetWBP_QuestList _mainwidget))
  (LocalVariables|SetLocalQuestClass QuestClass)
  (LocalVariables|SetLocalShouldStartImmediately ShouldStartImmediately)
  (if (and (Utilities|IsValidClass QuestClass) (not (Utilities|Array|ContainsItem (Variables|QuestSystem|GetAllQuestClasses) QuestClass)))
    (Utilities|Array|Add (Variables|QuestSystem|GetAllQuestClasses) (LocalVariables|GetLocalQuestClass))
    (bind _returnvalue (Game|SpawnActorfromClass (LocalVariables|GetLocalQuestClass) (Math|Transform|MakeTransform "0, 0, 0" "0, 0, 0" "1,1,1") "AlwaysSpawn" 0 0))
    (bind _output_get (LocalVariables|SetLocalQuestActor _returnvalue))
    (Utilities|Array|Add (Variables|QuestSystem|GetCurrentQuestActors) _output_get)
    (Default|InitStartingGoals _output_get)
    (bind _questwidget (Default|AddQuest (Variables|/Game/QuestSystem/Widgets/WBP_MainWidget.WBP_MainWidget_C|GetWBP_QuestList (Variables|UI|GetMainWidget)) (LocalVariables|GetLocalQuestActor)))
    (bind _output_get_2 (Variables|/Game/QuestSystem/Blueprints/Actors/QuestActors/BP_QuestMaster.BP_QuestMaster_C|SetQuestWidget (LocalVariables|GetLocalQuestActor) _questwidget))
    (Default|UpdateQuest _output_get_2)
    (if (or (LocalVariables|GetLocalShouldStartImmediately) (<= (Utilities|Array|Length (Variables|QuestSystem|GetCurrentQuestActors)) 1))
      (CallFunction|SelectNewQuest (LocalVariables|GetLocalQuestActor) (Utilities|Array|Get(acopy) (Variables|/Game/QuestSystem/Widgets/WBP_Quest.WBP_Quest_C|GetGoalWidgets (Variables|/Game/QuestSystem/Blueprints/Actors/QuestActors/BP_QuestMaster.BP_QuestMaster_C|GetQuestWidget (LocalVariables|GetLocalQuestActor)))))
      (if (Variables|/Game/QuestSystem/Widgets/WBP_QuestList.WBP_QuestList_C|GetIsSlidedOut _wbp_questlist)
        (UserInterface|Animation|PlayAnimation _wbp_questlist (Variables|/Game/QuestSystem/Widgets/WBP_QuestList.WBP_QuestList_C|GetSlideOut _wbp_questlist) 0.0 1 "Reverse" 1.0 false)
        (Variables|/Game/QuestSystem/Widgets/WBP_QuestList.WBP_QuestList_C|SetIsSlidedOut _wbp_questlist false)))
    (return true)
    (else
      (return false))))

(fn GetDistancetoGoal
  (bind _player (Variables|Player|GetPlayer))
  (bind _currentgoal (Variables|QuestSystem|GetCurrentGoal))
  (bind _goallocation (Utilities|Struct|BreakS_GoalInfo _currentgoal))
  (bind _returnvalue (Transformation|GetActorLocation _player))
  (return (Math|Float|Truncate (/ (Math|Vector|VectorLength (- (Math|Vector|MakeVector (.x _returnvalue) (.y _returnvalue) 0.0) (Math|Vector|MakeVector (.x (.location _goallocation)) (.y (.location _goallocation)) 0.0))) 1e+02))))

(fn UpdateDirectionArrow
  (Class|Widget|SetRenderTransformAngle (Variables|/Game/QuestSystem/Widgets/WBP_Minimap.WBP_Minimap_C|GetDirectionArrow (Variables|/Game/QuestSystem/Widgets/WBP_MainWidget.WBP_MainWidget_C|GetWBP_Minimap (Variables|UI|GetMainWidget))) (.yaw (Math|Rotator|FindLookatRotation (Transformation|GetActorLocation (Variables|Player|GetPlayer)) (.location (.GoalLocation (Utilities|Struct|BreakS_GoalInfo (Variables|QuestSystem|GetCurrentGoal))))))))