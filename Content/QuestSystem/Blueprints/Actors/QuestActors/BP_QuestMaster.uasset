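; Quest actor that tracks a quest's active and completed subgoals, using goal data from QuestInfo.
; Starting indices seed the active goals and description, and a separate function can step to a following index.
; CompleteGoal records a success, activates that goal's following subgoals for branching progression, and directly adds or removes WBP_Goal entries in the quest widget, reselecting if needed.
; The event graph and construction script are empty, so all logic runs through function calls.
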(event EventBeginPlay)

(event Collision|EventActorBeginOverlap
  (params (OtherActor :type Actor%20Object%20Reference)))

(event EventTick
  (params (DeltaSeconds :type Float%20%28single-precision%29)))

(fn ConstructionScript)

(fn UpdateSubgoals
  (Utilities|Array|Clear (Variables|ReadOnly|GetCurrentGoals))
  (for _array_element (Variables|ReadOnly|GetCurrentGoalIndices)
    (Utilities|Array|Add (Variables|ReadOnly|GetCurrentGoals) (Utilities|Array|Get(acopy) (.Goals (Utilities|Struct|BreakS_QuestInfo (Variables|Quest|GetQuestInfo))) _array_element)))
  (return))

(fn InitStartingGoals
  (Utilities|Array|Clear (Variables|ReadOnly|GetCurrentGoalIndices))
  (Variables|ReadOnly|SetCurrentGoalIndices (Variables|Quest|GetStartingGoalIndices))
  (CallFunction|UpdateSubgoals)
  (Variables|ReadOnly|SetCurrentDescription (Utilities|Struct|BreakS_QuestInfo (Variables|Quest|GetQuestInfo))))

(fn GotoNextSubgoal
  (bind _questinfo (Variables|Quest|GetQuestInfo))
  (bind _currentgoalindices (Variables|ReadOnly|GetCurrentGoalIndices))
  (bind _currentgoalindices_2 (Variables|ReadOnly|GetCurrentGoalIndices))
  (bind _goals (Utilities|Struct|BreakS_QuestInfo _questinfo))
  (bind _maxvalue (Math|Integer|MaxOfIntArray _currentgoalindices))
  (bind _returnvalue (Utilities|Array|LastIndex _goals))
  (bind _returnvalue_2 (+ _maxvalue 1))
  (bind _returnvalue_3 (<= _returnvalue_2 _returnvalue))
  (if _returnvalue_3
    (Utilities|Array|Clear _currentgoalindices_2)
    (bind _output_get (LocalVariables|SetNextIndex _returnvalue_2))
    (Utilities|Array|Add _currentgoalindices_2 _output_get)
    (CallFunction|UpdateSubgoals))
  (return _returnvalue_3))

(fn CompleteGoal
  (params (CompletedGoalIndex :type Integer))
  (bind _questwidget (Variables|UI|GetQuestWidget))
  (bind _questwidget_2 (Variables|UI|GetQuestWidget))
  (bind _questwidget_3 (Variables|UI|GetQuestWidget))
  (bind _goalwidgets (Variables|/Game/QuestSystem/Widgets/WBP_Quest.WBP_Quest_C|GetGoalWidgets _questwidget))
  (bind _output_get (LocalVariables|SetLocalCompletedGoalIndex CompletedGoalIndex))
  (if (Utilities|Array|ContainsItem (Variables|ReadOnly|GetCurrentGoalIndices) _output_get)
    (bind _output_get_2 (LocalVariables|SetLocalCompletedGoal (Utilities|Array|Get(acopy) (Variables|ReadOnly|GetCurrentGoals) (LocalVariables|GetLocalCompletedGoalIndex))))
    (Utilities|Array|Add (Variables|ReadOnly|GetCompletedGoals) (Utilities|Struct|MakeS_CompletedGoal (LocalVariables|GetLocalCompletedGoalIndex) _output_get_2 true))
    (Utilities|Array|RemoveItem (Variables|ReadOnly|GetCurrentGoals) (LocalVariables|GetLocalCompletedGoal))
    (LocalVariables|SetLocalWidgetIndex (Utilities|Array|FindItem (Variables|ReadOnly|GetCurrentGoalIndices) (LocalVariables|GetLocalCompletedGoalIndex)))
    (Utilities|Array|RemoveItem (Variables|ReadOnly|GetCurrentGoalIndices) (LocalVariables|GetLocalCompletedGoalIndex))
    (Widget|RemovefromParent (Utilities|Array|Get(acopy) _goalwidgets (LocalVariables|GetLocalWidgetIndex)))
    (Utilities|Array|RemoveIndex _goalwidgets (LocalVariables|GetLocalWidgetIndex))
    (for _array_element (Utilities|Struct|BreakS_GoalInfo (LocalVariables|GetLocalCompletedGoal))
      (Utilities|Array|Add (Variables|ReadOnly|GetCurrentGoalIndices) _array_element)
      (Utilities|Array|Add (Variables|ReadOnly|GetCurrentGoals) (Utilities|Array|Get(acopy) (Utilities|Struct|BreakS_QuestInfo (Variables|Quest|GetQuestInfo)) _array_element))
      (bind _returnvalue (UserInterface|CreateWidget "/Game/QuestSystem/Widgets/WBP_Goal.WBP_Goal_C" 0 (Utilities|Array|Get(acopy) (Utilities|Struct|BreakS_QuestInfo (Variables|Quest|GetQuestInfo)) _array_element) self _questwidget_2))
      (Utilities|Array|Add (Variables|/Game/QuestSystem/Widgets/WBP_Quest.WBP_Quest_C|GetGoalWidgets _questwidget_2) _returnvalue)
      (Widget|Panel|AddChild (Variables|/Game/QuestSystem/Widgets/WBP_Quest.WBP_Quest_C|GetGoalsBox _questwidget_2) _returnvalue))
    (if (== (Variables|ReadOnly|GetSelectedSubgoalIndex) (LocalVariables|GetLocalCompletedGoalIndex))
      (Default|SelectGoal _questwidget_3 (Utilities|Array|Get(acopy) (Variables|/Game/QuestSystem/Widgets/WBP_Quest.WBP_Quest_C|GetGoalWidgets _questwidget_3))))
    (return true)
    (else
      (return false))))