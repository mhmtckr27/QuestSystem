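; Player character Blueprint for a quest system that tracks the player's level and experience.
; On BeginPlay it spawns a quest manager, creates the main HUD widget linked to it, and initializes the avatar's level and EXP display.
; UpdateEXP loops to carry overflow across multiple level-ups, while LevelUp scales the next EXP requirement by a multiplier and plays a sound and particle effect.
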(event EventBeginPlay
  (bind _returnvalue (Game|SpawnActorfromClass "/Game/QuestSystem/Blueprints/Actors/BP_QuestManager.BP_QuestManager_C" (Math|Transform|MakeTransform "0, 0, 0" "0, 0, 0" "1,1,1") "AlwaysSpawn" 0 self 0))
  (bind _output_get (Variables|QuestSystem|SetQuestManager _returnvalue))
  (bind _returnvalue_2 (UserInterface|CreateWidget "/Game/QuestSystem/Widgets/WBP_MainWidget.WBP_MainWidget_C" 0 _output_get))
  (bind _output_get_2 (Variables|UI|SetMainWidget _returnvalue_2))
  (Variables|/Game/QuestSystem/Blueprints/Actors/BP_QuestManager.BP_QuestManager_C|SetMainWidget (Variables|QuestSystem|GetQuestManager) _output_get_2)
  (UserInterface|Viewport|AddtoViewport _output_get_2 0)
  (Default|OnLevelUpdate (Variables|/Game/QuestSystem/Widgets/WBP_MainWidget.WBP_MainWidget_C|GetWBP_PlayerAvatar (Variables|UI|GetMainWidget)) (Variables|ExperienceSystem|GetCurrentLevel))
  (Default|OnEXPUpdate (Variables|/Game/QuestSystem/Widgets/WBP_MainWidget.WBP_MainWidget_C|GetWBP_PlayerAvatar (Variables|UI|GetMainWidget)) (Variables|ExperienceSystem|GetCurrentEXP) (Variables|ExperienceSystem|GetEXPNeededForNextLevel)))

(event Collision|EventActorBeginOverlap
  (params (OtherActor :type Actor%20Object%20Reference)))

(event EventTick
  (params (DeltaSeconds :type Float%20%28single-precision%29)))

(fn ConstructionScript
  (|CallParentFunction))

(fn UpdateEXP
  (params (EXPChange :type Integer))
  (bind _output_get (Variables|ExperienceSystem|SetCurrentEXP (+ EXPChange (Variables|ExperienceSystem|GetCurrentEXP))))
  (if (< _output_get (Variables|ExperienceSystem|GetEXPNeededForNextLevel)) :!label _label
    (Default|OnEXPUpdate (Variables|/Game/QuestSystem/Widgets/WBP_MainWidget.WBP_MainWidget_C|GetWBP_PlayerAvatar (Variables|UI|GetMainWidget)) (Variables|ExperienceSystem|GetCurrentEXP) (Variables|ExperienceSystem|GetEXPNeededForNextLevel))
    (else
      (Variables|ExperienceSystem|SetCurrentEXP (- (Variables|ExperienceSystem|GetCurrentEXP) (Variables|ExperienceSystem|GetEXPNeededForNextLevel)))
      (ExperienceSystem|LevelUp)
      (goto _label))))

(fn LevelUp
  (Utilities|FlowControl|Sequence
    (:then_0
      ;[1 1 1] Logic
      (bind _result (Math|Integer|IncrementInt (Variables|ExperienceSystem|GetCurrentLevel))
        (:%20%20
          (Default|OnLevelUpdate (Variables|/Game/QuestSystem/Widgets/WBP_MainWidget.WBP_MainWidget_C|GetWBP_PlayerAvatar (Variables|UI|GetMainWidget)) _result)
          (Variables|ExperienceSystem|SetEXPNeededForNextLevel (Math|Float|Truncate (* (Variables|ExperienceSystem|GetEXPNeededForNextLevel) (Variables|ExperienceSystem|GetNextLevelEXPMultiplier)))))))
    (:then_1
      ;[1 1 1] Effects
      (Audio|PlaySound2D "/Game/QuestSystem/Audio/LevelUpSound.LevelUpSound" 0.5 1.0 0.0 0 0)
      (Components|Activation|Activate (Variables|Default|GetLevelUpParticle) true))))