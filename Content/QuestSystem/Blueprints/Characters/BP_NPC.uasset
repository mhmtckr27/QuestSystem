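; BP_NPC is a quest-giving NPC that shows a name widget and a quest icon.
; On BeginPlay it sets the player character as owner, fills the interaction widget's name and shows the icon if HasQuest is true.
; Radius enter and exit events toggle the interaction widget.
; Interacting adds and immediately starts the hard-coded BP_Quest_Test1 through the character's QuestManager if absent, then hides the icon.
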(event EventBeginPlay
  (Actor|SetOwner (Game|GetPlayerCharacter 0))
  (bind _aswbp_interaction (Utilities|Casting|CastToWBP_Interaction (UserInterface|GetUserWidgetObject (Variables|Default|GetInteractionWidget))))
  (Rendering|Components|TextRender|SetText (Variables|/Game/QuestSystem/Widgets/WBP_Interaction.WBP_Interaction_C|GetName _aswbp_interaction) (Variables|Default|GetName))
  (Rendering|SetVisibility (Variables|Default|GetQuestIcon) (Variables|Default|GetHasQuest) false))

(event EventOnPlayerEnterRadius
  (params (Character :type BP%20Player%20Character%20Object%20Reference))
  (Rendering|SetVisibility (Variables|Default|GetInteractionWidget) true false))

(event EventOnPlayerExitRadius
  (params (Character :type BP%20Player%20Character%20Object%20Reference))
  (Rendering|SetVisibility (Variables|Default|GetInteractionWidget) false false))

(event EventOnInteract
  (params (Character :type BP%20Player%20Character%20Object%20Reference))
  (bind _questmanager (Variables|/Game/QuestSystem/Blueprints/Characters/BP_PlayerCharacter.BP_PlayerCharacter_C|GetQuestManager Character))
  (if (not (Utilities|Array|ContainsItem (Variables|/Game/QuestSystem/Blueprints/Actors/BP_QuestManager.BP_QuestManager_C|GetAllQuestClasses _questmanager) "/Game/QuestSystem/Blueprints/Actors/QuestActors/BP_Quest_Test1.BP_Quest_Test1_C"))
    (Default|AddNewQuest _questmanager "/Game/QuestSystem/Blueprints/Actors/QuestActors/BP_Quest_Test1.BP_Quest_Test1_C" true)
    (Rendering|SetVisibility (Variables|Default|GetQuestIcon) false false)))

(fn ConstructionScript)