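; Player controller for the quest system that shows the cursor and sets Game and UI input focused on the player character's main widget.
; Debug keys grant EXP, add a test quest and complete the current quest's first goal through the character and its QuestManager.
; E messages interactable actors overlapping the character's interaction capsule.
; J toggles the quest list slide animation, reversing it mid-play, when any quests exist.
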(event EventBeginPlay
  (Input|SetInputModeGameandUI (Game|GetPlayerController 0) (Variables|/Game/QuestSystem/Blueprints/Characters/BP_PlayerCharacter.BP_PlayerCharacter_C|GetMainWidget (.AsBP%20Player%20Character (Utilities|Casting|CastToBP_PlayerCharacter (Game|GetPlayerCharacter 0)))) "DoNotLock" false)
  (Variables|Default|SetbShowMouseCursor true))

(event Input|KeyboardEvents|1
  (params (Key :type Key%20Structure :default "None"))
  ;[1 1 1] DEBUG: 1 to Update EXP
  (:Pressed
    (Default|UpdateEXP (.AsBP%20Player%20Character (Utilities|Casting|CastToBP_PlayerCharacter (Game|GetPlayerCharacter 0))) 5000)))

(event Input|KeyboardEvents|2
  (params (Key :type Key%20Structure :default "None"))
  ;[1 1 1] DEBUG: 2 to Give Quest
  (:Pressed
    (Default|AddNewQuest (Variables|/Game/QuestSystem/Blueprints/Characters/BP_PlayerCharacter.BP_PlayerCharacter_C|GetQuestManager (.AsBP%20Player%20Character (Utilities|Casting|CastToBP_PlayerCharacter (Game|GetPlayerCharacter 0)))) "/Game/QuestSystem/Blueprints/Actors/QuestActors/BP_Quest_Test2.BP_Quest_Test2_C" true)))

(event Input|KeyboardEvents|E
  (params (Key :type Key%20Structure :default "None"))
  ;[1 1 1] DEBUG: E to Interact (Talk)
  (:Pressed
    (bind _array_element (Utilities|Array|ForEachLoopwithBreak (Collision|GetOverlappingActors (Variables|/Game/QuestSystem/Blueprints/Characters/BP_PlayerCharacter.BP_PlayerCharacter_C|GetInteractionCapsule (.AsBP%20Player%20Character (Utilities|Casting|CastToBP_PlayerCharacter (Game|GetPlayerCharacter 0)))) 0 :!class /Script/Engine.PrimitiveComponent))
      (:LoopBody
        (if (Utilities|DoesObjectImplementInterface _array_element "/Game/QuestSystem/Blueprints/Interfaces/I_Interactable.I_Interactable_C")
          (Class|IInteractable|OnInteract(Message) _array_element (.AsBP%20Player%20Character (Utilities|Casting|CastToBP_PlayerCharacter (Game|GetPlayerCharacter 0)))))))))

(event Input|KeyboardEvents|J
  (params (Key :type Key%20Structure :default "None"))
  (bind _returnvalue (Game|GetPlayerCharacter 0))
  (bind _asbp_player_character (Utilities|Casting|CastToBP_PlayerCharacter _returnvalue))
  (bind _mainwidget (Variables|/Game/QuestSystem/Blueprints/Characters/BP_PlayerCharacter.BP_PlayerCharacter_C|GetMainWidget _asbp_player_character))
  (bind _wbp_questlist (Variables|/Game/QuestSystem/Widgets/WBP_MainWidget.WBP_MainWidget_C|GetWBP_QuestList _mainwidget))
  (bind _slideout (Variables|/Game/QuestSystem/Widgets/WBP_QuestList.WBP_QuestList_C|GetSlideOut _wbp_questlist))
  ;[1 1 1] DEBUG: J to Show/Hide Quest List
  (:Pressed
    (if (> (Utilities|Array|Length (Variables|/Game/QuestSystem/Blueprints/Actors/BP_QuestManager.BP_QuestManager_C|GetAllQuestClasses (Variables|/Game/QuestSystem/Blueprints/Characters/BP_PlayerCharacter.BP_PlayerCharacter_C|GetQuestManager _asbp_player_character))) 0)
      (if (Class|UserWidget|IsAnimationPlaying _wbp_questlist _slideout)
        (Class|UserWidget|ReverseAnimation _wbp_questlist _slideout)
        (else
          (UserInterface|Animation|PlayAnimation _wbp_questlist _slideout 0.0 1 (select (Variables|/Game/QuestSystem/Widgets/WBP_QuestList.WBP_QuestList_C|GetIsSlidedOut _wbp_questlist) "Reverse" "Forward") 1.0 false)))
      (Variables|/Game/QuestSystem/Widgets/WBP_QuestList.WBP_QuestList_C|SetIsSlidedOut _wbp_questlist (not (Variables|/Game/QuestSystem/Widgets/WBP_QuestList.WBP_QuestList_C|GetIsSlidedOut _wbp_questlist))))))

(event Input|KeyboardEvents|3
  (params (Key :type Key%20Structure :default "None"))
  ;[1 1 1] DEBUG: Complete first goal
  (:Pressed
    (Default|CompleteGoal (Variables|/Game/QuestSystem/Blueprints/Actors/BP_QuestManager.BP_QuestManager_C|GetCurrentQuest (Variables|/Game/QuestSystem/Blueprints/Characters/BP_PlayerCharacter.BP_PlayerCharacter_C|GetQuestManager (.AsBP%20Player%20Character (Utilities|Casting|CastToBP_PlayerCharacter (Game|GetPlayerCharacter 0))))))))

(fn ConstructionScript)